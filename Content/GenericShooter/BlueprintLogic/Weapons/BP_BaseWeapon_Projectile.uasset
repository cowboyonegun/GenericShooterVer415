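; Base projectile weapon Blueprint that extends the parent weapon's Fire to spawn projectiles with server authority.
; Clients send a server fire event, and FireProjectile spawns ProjectileClass only on authority for replication to all clients.
; The projectile launches along the camera aim, offset past the owner's capsule radius to avoid spawning inside the player.
; It receives the pawn and controller as instigators, and its mesh ignores the shooter when moving.
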(event `self.Fire`
  ;[1 1 1] If client, tell server to fire. Do not spawn projectiles on the client.
  (`parent.Fire`)
  (`/Engine/EditorBlueprintResources/ActorMacros.Switch Has Authority` :!label _label
    (:`Authority`
      _)
    (:`Remote`
      (`self.ServerFireProjectile`)))
  (`self.FireProjectile`))

(event `ServerFireProjectile`
  ;[1 1 1] If client, tell server to fire. Do not spawn projectiles on the client.
  (goto _label))

(fn `FireProjectile`
  (bind _aim (`self.GetCameraAim` false))
  (bind _owningpawn (`self.OwningPawn`))
  (bind _returnvalue (`KismetMathLibrary.Normal` _aim))
  ;[1 1 1] Make sure we are on the server...
  (`/Engine/EditorBlueprintResources/ActorMacros.Switch Has Authority`
    (:`Authority`
      ;[1 1 1] Spawn the projectile. This actor will be replicated to all clients.
      (bind _returnvalue_2 (`|SpawnActorFromClass` (`self.ProjectileClass`) (`KismetMathLibrary.MakeTransform` (+ (`self.GetWeaponFireStartTraceLocation` _aim) (* _returnvalue (+ (`CapsuleComponent.CapsuleRadius` (`Character.CapsuleComponent` (`self.OwningPawn`))) 25.0))) (`/Game/GenericShooter/BlueprintLogic/BPML_Helpers.VectorToRotator` _returnvalue)) "AlwaysSpawn" "OverrideRootScale" self _returnvalue (`/Game/GenericShooter/BlueprintLogic/BP_PlayerCharacter.GetCastedController` _owningpawn) _owningpawn))
      (`PrimitiveComponent.IgnoreActorWhenMoving` (`/Game/GenericShooter/BlueprintLogic/Weapons/BP_ProjectileBase.Mesh` _returnvalue_2) _owningpawn true)
      (return))
    (:`Remote`
      (return))))

(fn `UserConstructionScript`
  (`parent.UserConstructionScript`))