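; Weapon impact effect actor that spawns a particle, sound and attached decal matched to the physical surface that was hit.
; On BeginPlay it reads the surface from HitInfo, falling back to default, and selects that surface's effect set.
; Unloaded soft references are async loaded, then the spawn retries.
; LoadAllAssets async loads assets for every surface type, and the construction script enables auto-destroy when finished.
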(event `self.ReceiveBeginPlay`
  (`|ExecutionSequence`
    (:`then_0`
      (bind (_bwasloaded _effectid) (`self.SpawnParticleEffect` :!label _label))
      (if (not _bwasloaded)
        (`|LoadAsset` _effectid)
        (goto _label)))
    (:`then_1`
      (bind (_bwasloaded_2 _soundid) (`self.SpawnSound` :!label _label_2))
      (if (not _bwasloaded_2)
        (`|LoadAsset` _soundid)
        (goto _label_2)))
    (:`then_2`
      (bind (_bwasloaded_3 _decaldata) (`self.SpawnDecal` :!label _label_3))
      (if (not _bwasloaded_3)
        (`|LoadAsset` (`.Material_9_7D58DFBD4EC3FF3331597E9F6C7605A3` (break `/Game/GenericShooter/BlueprintLogic/Weapons/FDecalData` _decaldata)))
        (goto _label_3)))))

(event `LoadAllAssets`
  (bind _enumvalue (foreach `EPhysicalSurface`)
    (:`LoopBody`
      (`|ExecutionSequence`
        (:`then_0`
          (bind (_effect _sound _decal) (break `/Game/GenericShooter/BlueprintLogic/Weapons/FPhysicalMaterialEffectInfo` (`self.GetPhysMatInfo` _enumvalue)))
          (`|LoadAsset` _effect))
        (:`then_1`
          (`|LoadAsset` _sound))
        (:`then_2`
          (`|LoadAsset` (`.Material_9_7D58DFBD4EC3FF3331597E9F6C7605A3` (break `/Game/GenericShooter/BlueprintLogic/Weapons/FDecalData` _decal))))))))

(fn `GetImpactSurfaceType`
  (returns (SurfaceType :type "EPhysicalSurface Enum"))
  (bind (_bblockinghit _binitialoverlap _time _location _impactpoint _normal _impactnormal _physmat) (`GameplayStatics.BreakHitResult` (`self.HitInfo`)))
  (return (select `bool` (`KismetSystemLibrary.IsValid` _physmat) :`false` "SurfaceType_Default" :`true` (`PhysicalMaterial.SurfaceType` _physmat))))

(fn `GetPhysMatInfo`
  (params (SurfaceType :type "EPhysicalSurface Enum"))
  (returns (Info :type "/Game/GenericShooter/BlueprintLogic/Weapons/FPhysicalMaterialEffectInfo Structure"))
  (return (select `EPhysicalSurface` SurfaceType :`SurfaceType_Default` (`self.Default`) :`SurfaceType1` (`self.Concrete`) :`SurfaceType2` (`self.Dirt`) :`SurfaceType3` (`self.Water`) :`SurfaceType4` (`self.Metal`) :`SurfaceType5` (`self.Wood`) :`SurfaceType6` (`self.Grass`) :`SurfaceType7` (`self.Glass`) :`SurfaceType8` (`self.Flesh`))))

(fn `SpawnDecal`
  (returns (bWasLoaded :type Boolean) (DecalData :type "/Game/GenericShooter/BlueprintLogic/Weapons/FDecalData Structure"))
  (bind (_bblockinghit _binitialoverlap _time _location _impactpoint _normal _impactnormal _physmat _hitactor _hitcomponent _hitbonename) (`GameplayStatics.BreakHitResult` (`self.HitInfo`)))
  (bind (_effect _sound _decal) (break `/Game/GenericShooter/BlueprintLogic/Weapons/FPhysicalMaterialEffectInfo` (`self.GetPhysMatInfo` (`self.GetImpactSurfaceType`))))
  (bind (_material _size _lifespan) (break `/Game/GenericShooter/BlueprintLogic/Weapons/FDecalData` _decal))
  (bind _object (`|ConvertAsset` _material))
  ;[1 1 1] Spawn Decal if valid
  (`/Engine/EditorBlueprintResources/StandardMacros.IsValid` _object
    (:`Is Valid`
      (`GameplayStatics.SpawnDecalAttached` _object (`KismetMathLibrary.MakeVector` 1.0 _size _size) _hitcomponent _hitbonename _impactpoint (`/Game/GenericShooter/BlueprintLogic/BPML_Helpers.VectorToRotator` _impactnormal) "KeepWorldPosition" _lifespan)
      (return true _decal))
    (:`Is Not Valid`
      (return false _decal))))

(fn `SpawnParticleEffect`
  (returns (bWasLoaded :type Boolean) (EffectID :type "ParticleSystem Object Reference"))
  (bind _effect (break `/Game/GenericShooter/BlueprintLogic/Weapons/FPhysicalMaterialEffectInfo` (`self.GetPhysMatInfo` (`self.GetImpactSurfaceType`))))
  (bind _object (`|ConvertAsset` _effect))
  ;[1 1 1] Spawn Particle Effect if effect is valid
  (`/Engine/EditorBlueprintResources/StandardMacros.IsValid` _object
    (:`Is Valid`
      (`GameplayStatics.SpawnEmitterAtLocation` _object (`self.K2_GetActorLocation`) (`/Game/GenericShooter/BlueprintLogic/BPML_Helpers.VectorToRotator` (`.ImpactNormal` (`GameplayStatics.BreakHitResult` (`self.HitInfo`)))))
      (return true _effect))
    (:`Is Not Valid`
      (return false _effect))))

(fn `SpawnSound`
  (returns (bWasLoaded :type Boolean) (SoundID :type "SoundCue Object Reference"))
  (bind (_effect _sound) (break `/Game/GenericShooter/BlueprintLogic/Weapons/FPhysicalMaterialEffectInfo` (`self.GetPhysMatInfo` (`self.GetImpactSurfaceType`))))
  (bind _object (`|ConvertAsset` _sound))
  ;[1 1 1] Spawn Sound if valid
  (`/Engine/EditorBlueprintResources/StandardMacros.IsValid` _object
    (:`Is Valid`
      (`GameplayStatics.PlaySoundAtLocation` _object (`self.K2_GetActorLocation`))
      (return true _sound))
    (:`Is Not Valid`
      (return false _sound))))

(fn `UserConstructionScript`
  (set `self.bAutoDestroyWhenFinished` true))