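; Ammo pickup actor that refills the interacting pawn's weapon of a matching WeaponType.
; It is always focusable, highlighting its mesh via custom depth only for the locally controlled pawn and showing a tooltip for pickup, max ammo, or no suitable weapon.
; Pickup is allowed when that weapon is below max ammo; the server adds the configured ammo and destroys the actor.
; Construction applies an optional override material.
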(event `/Game/GenericShooter/BlueprintLogic/Interfaces/BPI_Pickupable.SetFocused`
  (params (InteractingPawn :type "/Game/GenericShooter/BlueprintLogic/BP_PlayerCharacter Object Reference") (IsFocused :type Boolean))
  (`PrimitiveComponent.SetRenderCustomDepth` (`self.StaticMesh`) (and (`Pawn.IsLocallyControlled` InteractingPawn) IsFocused)))

(fn `GetTooltipText`
  (params (OwningPawn :type "/Game/GenericShooter/BlueprintLogic/BP_PlayerCharacter Object Reference"))
  (returns (TooltipText :type Text))
  (bind (_hasweapon _theweapon) (`/Game/GenericShooter/BlueprintLogic/BP_PlayerCharacter.HasWeaponOfType` OwningPawn (`self.WeaponType`)))
  (bind _displayname (`/Game/GenericShooter/BlueprintLogic/Weapons/BP_BaseWeapon.DisplayName` _theweapon))
  ;[1 1 1] Make sure we have a weapon that would accept this ammo pickup...
  (if _hasweapon
    ;[1 1 1] Return a tooltip text that is relevant to the user's current ammo count for their weapon
    (return (select `bool` (< (`/Game/GenericShooter/BlueprintLogic/Weapons/BP_BaseWeapon.CurrentAmmo` _theweapon) (`/Game/GenericShooter/BlueprintLogic/Weapons/BP_BaseWeapon.MaxAmmo` _theweapon)) :`false` (`|FormatText` "Already Have Max Ammo For {WeaponName}" _displayname) :`true` (`|FormatText` "Press {Interact} To Pickup {WeaponName} Ammo" "E" _displayname)))
    (else
      (return (`|FormatText` "You Don't Have A Suitable Weapon For This Ammo")))))

(fn `IsFocusable`
  (params (OwningPawn :type "/Game/GenericShooter/BlueprintLogic/BP_PlayerCharacter Object Reference"))
  (returns (bFocusable :type Boolean))
  (return true))

(fn `IsPickupable`
  (params (InteractingPawn :type "/Game/GenericShooter/BlueprintLogic/BP_PlayerCharacter Object Reference"))
  (returns (CanPickup :type Boolean))
  (bind (_hasweapon _theweapon) (`/Game/GenericShooter/BlueprintLogic/BP_PlayerCharacter.HasWeaponOfType` InteractingPawn (`self.WeaponType`)))
  ;[1 1 1] Ammo is pickupable if player has weapon that needs ammo
  (if _hasweapon
    (return (< (`/Game/GenericShooter/BlueprintLogic/Weapons/BP_BaseWeapon.CurrentAmmo` _theweapon) (`/Game/GenericShooter/BlueprintLogic/Weapons/BP_BaseWeapon.MaxAmmo` _theweapon)))
    (else
      (return false))))

(fn `Pickup`
  (params (InteractingPawn :type "/Game/GenericShooter/BlueprintLogic/BP_PlayerCharacter Object Reference"))
  (returns (bPickedUp :type Boolean))
  (bind (_hasweapon _theweapon) (`/Game/GenericShooter/BlueprintLogic/BP_PlayerCharacter.HasWeaponOfType` InteractingPawn (`self.WeaponType`)))
  ;[1 1 1] Make sure we're on the server and the player has a weapon
  (`/Engine/EditorBlueprintResources/ActorMacros.Switch Has Authority`
    (:`Authority`
      (if _hasweapon
        ;[1 1 1] Add ammo to weapon and destroy the pickup
        (`/Game/GenericShooter/BlueprintLogic/Weapons/BP_BaseWeapon.AddAmmo` _theweapon (`self.AmmoAmount`) (`self.bAddToClip`) (`self.bSkipMaxAmmoCheck`))
        (`self.K2_DestroyActor`)
        (return true)
        (else
          _)))
    (:`Remote`
      _))
  (return false))

(fn `UserConstructionScript`
  (bind _overridematerial (`self.OverrideMaterial`))
  (`parent.UserConstructionScript`)
  (`/Engine/EditorBlueprintResources/StandardMacros.IsValid` _overridematerial
    (:`Is Valid`
      (`PrimitiveComponent.SetMaterial` (`self.StaticMesh`) 0 _overridematerial))))